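; BP_HamsterCam is a top-down camera actor that follows the Hamster from above.
; On BeginPlay it points its camera component straight down.
; Each tick it snaps to the Hamster's X and Y, raised by HeightVariable, with a fixed rotation and no smoothing.
; An unused, disconnected variant leads the position by a fraction of the Hamster's velocity, alongside leftover debug prints.
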(event `self.ReceiveBeginPlay`
  (`SceneComponent.K2_SetWorldRotation` (`self.CameraComponent`) (struct :`Pitch` -90.0) false false))

(event `self.ReceiveTick`
  (params (DeltaSeconds :type "Float (single-precision)"))
  (bind (_returnvalue_x _returnvalue_y _returnvalue_z) (`KismetMathLibrary.BreakVector` (`self.K2_GetActorLocation` (`self.Hamster`))))
  ;[1 1 1] Follow player
  (`self.K2_SetActorLocationAndRotation` (`KismetMathLibrary.MakeVector` _returnvalue_x _returnvalue_y (+ _returnvalue_z (`self.Height Variable`))) (struct :`Pitch` -90.0)))

(fn `UserConstructionScript`)